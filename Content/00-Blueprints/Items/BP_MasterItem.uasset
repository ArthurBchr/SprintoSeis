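; BP_MasterItem is an item Blueprint that shows a decal outline while it is being looked at as an interactable.
; The start-look event passes through a DoOnce to unhide DecalOutline, and the stop-look event resets that gate and hides it, each printing a debug string.
; The construction script applies DecalSize and ShapeScale as world scales on the decal and SMShape components.
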(event Custom|EnableOutline
  (Development|SetHiddeninGame (Variables|Default|GetDecal_Outline) false false))

(event Custom|DisableOutline
  (Development|SetHiddeninGame (Variables|Default|GetDecal_Outline) true false))

(event EventBeginPlay)

(event EventStartLookatInteractables
  (Utilities|FlowControl|DoOnce false
    (:Completed
      (CallFunction|EnableOutline)
      (Development|PrintString "enable"))))

(event EventStopLookatInteractables
  (Utilities|FlowControl|Sequence
    (:then_0
      (Utilities|FlowControl|DoOnce false) ; enters at Reset
    )
    (:then_1
      (CallFunction|DisableOutline)
      (Development|PrintString "disable"))))

(fn ConstructionScript
  (Transformation|SetWorldScale3D (Variables|Default|GetDecal_Outline) (Variables|00-GlobalParams|GetDecalSize))
  (Transformation|SetWorldScale3D (Variables|Default|GetSM_Shape) (Variables|00-GlobalParams|GetShapeScale)))