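; BP_TriggerEnding is a trigger actor that ends the game when the player reaches it.
; When a BP_FPSPlayer overlaps its sphere, it calls Ending on the player's indicator widget, destroys the player actor, and plays a Level Sequence.
; When the sequence finishes, the bound event opens the MainMenu level.
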(event OnComponentBeginOverlap(Sphere)
  (params (OverlappedComponent :type Primitive%20Component%20Object%20Reference) (OtherActor :type Actor%20Object%20Reference) (OtherComp :type Primitive%20Component%20Object%20Reference) (OtherBodyIndex :type Integer) (bFromSweep :type Boolean) (SweepResult :type Hit%20Result%20Structure%20%28by%20ref%29))
  (bind _asbp_fpsplayer (Utilities|Casting|CastToBP_FPSPlayer OtherActor))
  (Default|Ending (Variables|/Game/00-Blueprints/Player/BP_FPSPlayer.BP_FPSPlayer_C|GetWBP%20ref%20indicator _asbp_fpsplayer))
  (Actor|DestroyActor _asbp_fpsplayer)
  (bind _outactor (Sequencer|Player|CreateLevelSequencePlayer (Variables|Default|Getlvl%20sequencer)))
  (Sequencer|Player|Play (Variables|/Script/LevelSequence.LevelSequenceActor|GetSequencePlayer _outactor) :!class /Script/MovieScene.MovieSceneSequencePlayer)
  (EventDispatchers|BindEventtoOnFinished (Variables|/Script/LevelSequence.LevelSequenceActor|GetSequencePlayer _outactor) (delegate Custom|finished)))

(event Custom|finished
  (Game|OpenLevel(byObjectReference) "/Game/01-Maps/MainMenu.MainMenu"))

(event EventBeginPlay)

(event Collision|EventActorBeginOverlap
  (params (OtherActor :type Actor%20Object%20Reference)))

(event EventTick
  (params (DeltaSeconds :type Float%20%28single-precision%29)))

(fn ConstructionScript)